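; BP_PlayerController_UI is a player controller that manages the rings-collected status bar and an in-game menu.
; On BeginPlay it creates both widgets and adds only the status bar to the viewport.
; The keyboard menu action, if the menu is not already open, stops the ball pawn, shows and focuses the menu, and switches to UI-only input.
; Nothing here closes the menu or resets MenuOpened, and the end-level status bar removal is unconnected.
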(event EventBeginPlay
  ;[1 1 1] UI Setup on Start
  (Development|PrintString "Player Controller working")
  (bind _returnvalue (UserInterface|CreateWidget "/Game/Blueprints/UI/BP_UI_RingsCollected.BP_UI_RingsCollected_C"))
  (bind _output_get (Variables|Default|SetStatusBar _returnvalue))
  (UserInterface|Viewport|AddtoViewport _output_get 0)
  (bind _returnvalue_2 (UserInterface|CreateWidget "/Game/Blueprints/UI/BP_UI_Menu.BP_UI_Menu_C"))
  (Variables|Default|SetMenuReference _returnvalue_2))

(event Input|ActionEvents|InputActionMenuToggleKexboard
  (params (Key :type Key%20Structure))
  (bind _menureference (Variables|Default|GetMenuReference))
  ;[1 1 1] Closing and opening the menu on PC
  (:Pressed
    (if (not (Variables|Default|GetMenu%20Opened))
      (bind _asbp_normal_ball_pawn (Utilities|Casting|CastToBP_normalBall_Pawn (Game|Player|GetPlayerPawn 0)))
      (Default|StopMovement _asbp_normal_ball_pawn)
      (UserInterface|Viewport|AddtoViewport _menureference 0)
      (Widget|SetKeyboardFocus _menureference)
      (Input|SetInputModeUIOnly (Game|GetPlayerController 0) _menureference "LockAlways")
      (Variables|Default|SetMenu%20Opened true))))

(fn ConstructionScript)